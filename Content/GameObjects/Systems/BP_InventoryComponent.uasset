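; Inventory component that creates a WBP_Inventory widget, adds it to the viewport on BeginPlay and sizes its Inventory array to the slot count.
; Items live in the widget's grid children, which are queried and updated through message calls.
; Adding fills the first free slot and removing clears the first occupied slot of the matching type.
; The Inventory array is never filled here, and adding shows only a false return.
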(event `self.ReceiveBeginPlay`
  (bind _returnvalue (`|CreateWidget` "/Game/GameObjects/UserInterface/WBP_Inventory.WBP_Inventory_C" null self))
  (bind _output_get (set `self.InventoryWidget` _returnvalue))
  (`UserWidget.AddToViewport` _output_get 0)
  (`self.F_PrepareInventory`))

(fn `F_AddToInventory`
  (params (Item :type "/Game/Structs/Struct_CheckListPlayer Structure"))
  (returns (Success :type Boolean))
  (for _index (range (`self.NrOfSlots`))
    (bind _returnvalue (`PanelWidget.GetChildAt` (`/Game/GameObjects/UserInterface/WBP_Inventory.GridPanel_264` (`self.InventoryWidget`)) _index))
    (bind _occupied (message `/Game/Interfaces/BPI_InventorySlot.IsOccupied?` _returnvalue))
    (if (not _occupied)
      (`|ExecutionSequence`
        (:`then_0`
          (break))
        (:`then_1`
          (message `/Game/Interfaces/BPI_InventorySlot.OccupySlot` _returnvalue true (`local.Item`))))))
  (return false))

(fn `F_PrepareInventory`
  (`KismetArrayLibrary.Array_Resize` (`self.Inventory`) (`self.NrOfSlots`)))

(fn `F_RemoveFromInventory`
  (params (ItemToRemove :type "/Game/Enums/Enum_Items Enum" :default "NewEnumerator0"))
  (for _array_element (`PanelWidget.GetAllChildren` (`/Game/GameObjects/UserInterface/WBP_Inventory.GridPanel_264` (`self.InventoryWidget`)))
    (bind _itemtype (message `/Game/Interfaces/BPI_InventorySlot.F_GetItemType` _array_element))
    (bind _occupied (message `/Game/Interfaces/BPI_InventorySlot.IsOccupied?` _array_element))
    (if (and (== _itemtype ItemToRemove) _occupied)
      (`|ExecutionSequence`
        (:`then_0`
          (break))
        (:`then_1`
          (message `/Game/Interfaces/BPI_InventorySlot.F_ClearSlot` _array_element))))))