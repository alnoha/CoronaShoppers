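; BP_Desinfector is an interactable disinfectant station that disinfects the interacting actor and shows its remaining supply on a widget bar.
; Box overlaps register and unregister it as the overlapping actor's interactable through message calls.
; Interact sends the disinfect message, drains a fixed clamped amount and updates the bar, with no check for an empty supply.
; FGetDesinfectant is a stub that always returns zero.
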(event `self.ReceiveBeginPlay`
  (bind _aswbp_desinfection_remaining (cast `/Game/GameObjects/UserInterface/WBP_DesinfectionRemaining` (`WidgetComponent.GetUserWidgetObject` (`self.Bar`))))
  (set `self.DesinfectionRemainingWidget` _aswbp_desinfection_remaining))

(event `/Game/Interfaces/BPI_Interactable.Interact`
  (params (Interacting_Actor :type "Actor Object Reference"))
  (message `/Game/Interfaces/BPI_PLayer.F_Desinfect` Interacting_Actor)
  (bind _output_get (set `self.DesinfectantRemaining` (`KismetMathLibrary.FClamp` (- (`self.DesinfectantRemaining`) 0.2))))
  (`/Game/GameObjects/UserInterface/WBP_DesinfectionRemaining.UpdatePercentage` (`self.DesinfectionRemainingWidget`) _output_get))

(event `self.Box.OnComponentBeginOverlap`
  (params (OverlappedComponent :type "PrimitiveComponent Object Reference") (OtherActor :type "Actor Object Reference") (OtherComp :type "PrimitiveComponent Object Reference") (OtherBodyIndex :type Integer) (bFromSweep :type Boolean) (SweepResult :type "HitResult Structure (by ref)"))
  (message `/Game/Interfaces/BPI_PLayer.F_AddInteractable` OtherActor self))

(event `self.Box.OnComponentEndOverlap`
  (params (OverlappedComponent :type "PrimitiveComponent Object Reference") (OtherActor :type "Actor Object Reference") (OtherComp :type "PrimitiveComponent Object Reference") (OtherBodyIndex :type Integer))
  (message `/Game/Interfaces/BPI_PLayer.F_RemoveInteractable` OtherActor null))

(fn `F_GetDesinfectant`
  (returns (DesinfectantValue :type "Float (double-precision)"))
  (return 0.0))

(fn `UserConstructionScript`)