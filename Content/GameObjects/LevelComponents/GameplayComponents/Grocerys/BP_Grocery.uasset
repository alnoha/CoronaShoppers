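; BP_Grocery is an interactable grocery shelf actor that adds its grocery type to a character's inventory or takes it back out.
; A Box overlap registers it as the overlapping actor's interactable and, for the ThirdPersonCharacter, adds or removes the shelf on its inventory component.
; That component instantiates a widget on BeginPlay.
; Interact and put-back events send add and remove grocery messages to the interacting actor.
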(event `self.ReceiveBeginPlay`
  (`/Game/GameObjects/Systems/BP_GroceryInventoryComponent_2.InstanciateWidget` (`self.BP_GroceryInventoryComponent_2`) self))

(event `self.Box.OnComponentBeginOverlap`
  (params (OverlappedComponent :type "PrimitiveComponent Object Reference") (OtherActor :type "Actor Object Reference") (OtherComp :type "PrimitiveComponent Object Reference") (OtherBodyIndex :type Integer) (bFromSweep :type Boolean) (SweepResult :type "HitResult Structure (by ref)"))
  ;[1 1 1] Add/Remove Item from Character Interactable Variable
  (message `/Game/Interfaces/BPI_PLayer.F_AddInteractable` OtherActor self)
  (if (== (`GameplayStatics.GetObjectClass` OtherActor) "/Game/ThirdPersonBP/Blueprints/ThirdPersonCharacter.ThirdPersonCharacter_C")
    (`/Game/GameObjects/Systems/BP_GroceryInventoryComponent_2.AddShelf` (`self.BP_GroceryInventoryComponent_2`) self)))

(event `self.Box.OnComponentEndOverlap`
  (params (OverlappedComponent :type "PrimitiveComponent Object Reference") (OtherActor :type "Actor Object Reference") (OtherComp :type "PrimitiveComponent Object Reference") (OtherBodyIndex :type Integer))
  ;[1 1 1] Add/Remove Item from Character Interactable Variable
  (message `/Game/Interfaces/BPI_PLayer.F_RemoveInteractable` OtherActor null)
  (if (== (`GameplayStatics.GetObjectClass` OtherActor) "/Game/ThirdPersonBP/Blueprints/ThirdPersonCharacter.ThirdPersonCharacter_C")
    (`/Game/GameObjects/Systems/BP_GroceryInventoryComponent_2.RemoveShelf` (`self.BP_GroceryInventoryComponent_2`))))

(event `/Game/Interfaces/BPI_Interactable.Interact`
  (params (Interacting_Actor :type "Actor Object Reference"))
  ;[1 1 1] Add Grocery to Characters Inventory
  (message `/Game/Interfaces/BPI_PLayer.F_AddGrocery` Interacting_Actor (`self.GroceryType`)))

(event `/Game/Interfaces/BPI_Interactable.F_PutBack`
  (params (InteractingActor :type "Actor Object Reference"))
  (bind _grocerytype_items (break `/Game/Structs/Struct_CheckListPlayer` (`self.GroceryType`)))
  (message `/Game/Interfaces/BPI_PLayer.FRemoveGrocery` InteractingActor _grocerytype_items))

(fn `UserConstructionScript`)