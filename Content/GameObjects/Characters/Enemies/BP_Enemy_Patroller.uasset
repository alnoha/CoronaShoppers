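; Patrolling enemy Blueprint that endlessly walks between actors in its Destinations array, starting at BeginPlay.
; WalksRandomly selects either random destinations, bounded by TargetPoints minus one, or sequential cycling through a counted index.
; Each AI MoveTo, whether it succeeds or fails, leads to a pause, a Cough call and another pause before the next move.
; Sequential patrols randomize the first pause and wrap only once the index exceeds the destination count.
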(event `self.ReceiveBeginPlay`
  (`parent.ReceiveBeginPlay`)
  (for _ (`self.Destinations`)
    (set `self.CycleAmount` (+ (`self.CycleAmount`) 1)))
  (set `self.TargetsIndex` (- (`self.TargetPoints`) 1))
  (if (`self.WalksRandomly`)
    (`|AIMoveTo` self (0.0 0.0 0.0) (`|GetArrayItem` (`self.Destinations`) (`KismetMathLibrary.RandomInteger` (`self.TargetsIndex`))) 20.0 :!label _label
      (:`OnSuccess`
        _)
      (:`OnFail`
        _))
    (`KismetSystemLibrary.Delay` 1.0)
    (`self.Cough`)
    (`KismetSystemLibrary.Delay` 1.0)
    (goto _label)
    (else
      (`|AIMoveTo` self (0.0 0.0 0.0) (`|GetArrayItem` (`self.Destinations`) (`self.CycleIndex`)) 20.0 :!label _label_2
        (:`OnSuccess`
          _)
        (:`OnFail`
          _))
      (set `self.CycleIndex` (+ (`self.CycleIndex`) 1))
      (if (> (`self.CycleIndex`) (`self.CycleAmount`))
        (set `self.CycleIndex` 0))
      (`KismetSystemLibrary.Delay` (`KismetMathLibrary.RandomFloatInRange` 3.5 4.0))
      (`self.Cough`)
      (`KismetSystemLibrary.Delay` 1.0)
      (goto _label_2))))

(fn `UserConstructionScript`
  (`parent.UserConstructionScript`))