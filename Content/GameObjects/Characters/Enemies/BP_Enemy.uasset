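; Infectious enemy character that spreads coronavirus by spawning cough volumes from its mouth and flagging actors that overlap its aura as infected.
; BeginPlay builds a randomized rectangular route near the spawn and toggles the aura by class flag.
; WalkAround loops the SquarePartol macro, moving corner to corner with coughs between legs.
; A random Decide event picks cough, move, follow, wait or patrol, but nothing here triggers it or WalkAround.
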(event `self.ReceiveBeginPlay`
  (bind _aura (`self.Aura`))
  ;[1 0 0.04683] BeginPlay
  (`|ExecutionSequence`
    (:`then_0`
      (`KismetSystemLibrary.Delay` 0.05)
      (set `self.StartingPosition` (`self.K2_GetActorLocation`))
      (`ActorComponent.SetActive` (`self.Aura`) false false))
    (:`then_1`
      (set `self.WaitTime` 3.0))
    (:`then_2`
      (`self.SetSquarePartolRoute`))
    (:`then_3`
      ;[1 1 1] BOOL: Aura, Coughing.
      (if (`self.CoughingClass`)
        _))
    (:`then_4`
      (`KismetSystemLibrary.Delay` 0.1)
      (if (`self.AuraClass`)
        (`ActorComponent.Activate` _aura false)
        (else
          (`ActorComponent.Deactivate` _aura))))))

(event `Decide`
  ;[1 1 1] AI Decision Logic (Currently Random)
  (`KismetSystemLibrary.Delay` 2.0)
  (switch `int` (`KismetMathLibrary.RandomIntegerInRange` 0 4)
    (:`0`
      (`self.Cough`)
      (`KismetSystemLibrary.PrintString` "Cough"))
    (:`1`
      (`self.RandomMove`)
      (`KismetSystemLibrary.PrintString` "Move"))
    (:`2`
      (`self.FollowPlayer`)
      (`KismetSystemLibrary.PrintString` "Follow"))
    (:`3`
      (`self.Wait`)
      (`KismetSystemLibrary.PrintString` "Wait"))
    (:`4`
      (`self.Patroll`)
      (`KismetSystemLibrary.PrintString` "Patroll"))))

(event `WalkAround`
  ;[1 1 1] AI Walk in a Square
  (`self.SquarePartol` :!label _label
    (:`On Success`
      (goto _label))))

(event `FollowPlayer`
  ;[1 1 1] AI Follow Player Action
  (`|AIMoveTo` self (`self.K2_GetActorLocation` (`GameplayStatics.GetPlayerCharacter` 0)) null 100.0))

(event `TurnAround`
  (bind (_returnvalue_roll _returnvalue_pitch _returnvalue_yaw) (`KismetMathLibrary.BreakRotator` (`self.K2_GetActorRotation`)))
  ;[1 1 1] AI Turn Around Action
  (bind (_direction _turningalpha) (`Timeline|TL_Turning` :!via `PlayFromStart`)
    (:`Update`
      (`self.K2_SetActorRotation` (`KismetMathLibrary.MakeRotator` 0.0 0.0 (`KismetMathLibrary.Lerp` _returnvalue_yaw (`KismetMathLibrary.RandomFloatInRange` 0.0 180.0) _turningalpha))))))

(event `Cough`
  (bind _mesh (`self.Mesh`))
  ;[1 1 1] AI Cough Action
  (`|SpawnActorFromClass` "/Game/GameObjects/Characters/Enemies/BP_CoronaVolume.BP_CoronaVolume_C" (`KismetMathLibrary.MakeTransform` (`SceneComponent.GetSocketLocation` _mesh "mouth") (`KismetMathLibrary.MakeRotFromX` (`SceneComponent.GetForwardVector` _mesh))) "Undefined" "OverrideRootScale" null null))

(event `Wait`
  ;[1 1 1] AI Wait Action
  (`KismetSystemLibrary.Delay` (`self.WaitTime`)))

(event `RandomMove`
  ;[1 1 1] AI Move Action (Currently Random)
  (`|AIMoveTo` self (`NavigationSystemV1.K2_GetRandomReachablePointInRadius` (`self.K2_GetActorLocation`) 5000.0 null null) null))

(event `Patroll`
  ;[1 1 1] AI Patroll Action
  (`|AIMoveTo` self (`|GetArrayItem` (`|MakeArray` (`self.PositionOne`) (`self.PositionTwo`)) (`KismetMathLibrary.RandomInteger` 1)) null 100.0))

(event `self.Aura.OnComponentBeginOverlap`
  (params (OverlappedComponent :type "PrimitiveComponent Object Reference") (OtherActor :type "Actor Object Reference") (OtherComp :type "PrimitiveComponent Object Reference") (OtherBodyIndex :type Integer) (bFromSweep :type Boolean) (SweepResult :type "HitResult Structure (by ref)"))
  (message `/Game/Interfaces/BPI_PLayer.F_AddToInfectedStatus` OtherActor))

(fn `Set Patrol Route`
  (set `self.PositionOne` (`KismetMathLibrary.MakeVector` (`KismetMathLibrary.RandomFloatInRange` (`KismetMathLibrary.RandomFloatInRange` -1000.0 -500.0) (`KismetMathLibrary.RandomFloatInRange` 500.0 1000.0)) (`KismetMathLibrary.RandomFloatInRange` (`KismetMathLibrary.RandomFloatInRange` -1000.0 -500.0) (`KismetMathLibrary.RandomFloatInRange` 500.0 1000.0))))
  (set `self.PositionTwo` (`KismetMathLibrary.MakeVector` (`KismetMathLibrary.RandomFloatInRange` (`KismetMathLibrary.RandomFloatInRange` -1000.0 -500.0) (`KismetMathLibrary.RandomFloatInRange` 500.0 1000.0)) (`KismetMathLibrary.RandomFloatInRange` (`KismetMathLibrary.RandomFloatInRange` -1000.0 -500.0) (`KismetMathLibrary.RandomFloatInRange` 500.0 1000.0))))
  (set `self.PositionThree` (`KismetMathLibrary.MakeVector` (`KismetMathLibrary.RandomFloatInRange` (`KismetMathLibrary.RandomFloatInRange` -1000.0 -500.0) (`KismetMathLibrary.RandomFloatInRange` 500.0 1000.0)) (`KismetMathLibrary.RandomFloatInRange` (`KismetMathLibrary.RandomFloatInRange` -1000.0 -500.0) (`KismetMathLibrary.RandomFloatInRange` 500.0 1000.0))))
  (set `self.PositionFour` (`KismetMathLibrary.MakeVector` (`KismetMathLibrary.RandomFloatInRange` (`KismetMathLibrary.RandomFloatInRange` -1000.0 -500.0) (`KismetMathLibrary.RandomFloatInRange` 500.0 1000.0)) (`KismetMathLibrary.RandomFloatInRange` (`KismetMathLibrary.RandomFloatInRange` -1000.0 -500.0) (`KismetMathLibrary.RandomFloatInRange` 500.0 1000.0)))))

(fn `SetSquarePartolRoute`
  (bind (_returnvalue_x _returnvalue_y) (`KismetMathLibrary.BreakVector` (`self.K2_GetActorLocation`)))
  (bind _returnvalue (`KismetMathLibrary.RandomFloatInRange` 0.0 500.0))
  (bind _output_get (set `self.PositionOne` (`KismetMathLibrary.MakeVector` (+ _returnvalue_x _returnvalue) _returnvalue_y)))
  (bind _output_get_2 (set `self.PositionTwo` (`KismetMathLibrary.MakeVector` (.x _output_get) (- (.y _output_get) _returnvalue))))
  (bind _output_get_3 (set `self.PositionThree` (`KismetMathLibrary.MakeVector` (- (.x _output_get_2) _returnvalue) (.y _output_get_2))))
  (set `self.PositionFour` (`KismetMathLibrary.MakeVector` (.x _output_get_3) (+ (.y _output_get_3) _returnvalue))))

(fn `UserConstructionScript`)