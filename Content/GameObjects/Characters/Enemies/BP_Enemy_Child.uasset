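; BP_Enemy_Child is a child enemy character that endlessly wanders near its start point and coughs.
; From BeginPlay, RunAround uses AIMoveTo toward a random nearby X/Y offset, then calls Cough and pauses.
; RunBack returns it to StartingPosition and, after a short delay, restarts RunAround.
; Failed moves continue down the same path as successful ones, so the event-driven loop keeps going without Tick.
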(event `self.ReceiveBeginPlay`
  (`parent.ReceiveBeginPlay`)
  (`|ExecutionSequence`
    (:`then_0`
      (`self.RunAround`))))

(event `RunAround`
  (bind (_returnvalue_x _returnvalue_y) (`KismetMathLibrary.BreakVector` (`self.K2_GetActorLocation`)))
  (`|AIMoveTo` self (`KismetMathLibrary.MakeVector` (+ _returnvalue_x (`KismetMathLibrary.RandomFloatInRange` -200.0 200.0)) (+ _returnvalue_y (`KismetMathLibrary.RandomFloatInRange` -200.0 200.0))) null
    (:`OnSuccess`
      _)
    (:`OnFail`
      _))
  (`self.Cough`)
  (`KismetSystemLibrary.Delay` 1.0)
  (`self.RunBack`))

(event `RunBack`
  (`|AIMoveTo` self (`self.StartingPosition`) null
    (:`OnSuccess`
      _)
    (:`OnFail`
      _))
  (`KismetSystemLibrary.Delay` 0.2)
  (`self.RunAround`))

(fn `UserConstructionScript`
  (`parent.UserConstructionScript`))