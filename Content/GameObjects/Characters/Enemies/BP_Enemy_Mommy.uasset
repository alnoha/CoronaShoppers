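; BP_Enemy_Mommy is an enemy character that wanders between patrol points, coughing at each stop.
; On BeginPlay it runs the parent logic, calls SetPatrolRoute, then starts the WalkTowards loop.
; WalkTowards uses AIMoveTo toward a randomly picked position, then pauses, calls Cough and repeats, whether the move succeeds or fails.
; The random index covers only the first three of the four positions, so PositionFour is never chosen.
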(event `self.ReceiveBeginPlay`
  (`parent.ReceiveBeginPlay`)
  (`|ExecutionSequence`
    (:`then_0`
      (`self.Set Patrol Route`))
    (:`then_1`
      (`self.WalkTowards`))))

(event `WalkTowards`
  (`|AIMoveTo` self (`|GetArrayItem` (`|MakeArray` (`self.PositionOne`) (`self.PositionTwo`) (`self.PositionThree`) (`self.PositionFour`)) (`KismetMathLibrary.RandomInteger` 3)) null 100.0 :!label _label
    (:`OnSuccess`
      _)
    (:`OnFail`
      _))
  (`KismetSystemLibrary.Delay` 1.0)
  (`self.Cough`)
  (`KismetSystemLibrary.Delay` 1.0)
  (goto _label))

(fn `UserConstructionScript`
  (`parent.UserConstructionScript`))