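; Enemy manager Blueprint that spawns a single AI enemy when play begins.
; It randomly picks one of four spawn locations and a class from a Select of Child, OldPerson and Stander enemies.
; The random index has a hard-coded max of 2, so Stander is never chosen.
; GetEnemyClasses derives EnemyClassIndex from the class count, but the spawn does not use it.
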(event `self.ReceiveBeginPlay`
  (`self.GetEnemyClasses`)
  (`AIBlueprintHelperLibrary.SpawnAIFromClass` (select `int` (`KismetMathLibrary.RandomInteger` 2) :`0` "/Game/GameObjects/Characters/Enemies/BP_Enemy_Child.BP_Enemy_Child_C" :`1` "/Game/GameObjects/Characters/Enemies/BP_Enemy_OldPerson.BP_Enemy_OldPerson_C" :`2` "/Game/GameObjects/Characters/Enemies/BP_Enemy_Stander.BP_Enemy_Stander_C" :!type "Pawn Class Reference") null (`|GetArrayItem` (`|MakeArray` (`self.SpawnLocation1`) (`self.SpawnLocation2`) (`self.SpawnLocation3`) (`self.SpawnLocation4`)) (`KismetMathLibrary.RandomInteger` 4))))

(fn `GetEnemyClasses`
  (set `self.EnemyClassIndex` (- (`self.AmountOfEnemyClasses`) 1)))

(fn `UserConstructionScript`)